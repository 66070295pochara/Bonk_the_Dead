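; Corpse character that switches in and out of physics ragdoll and tracks its stunned and dragged states with gameplay tags.
; Damage stuns it unless it is being dragged, and releasing a drag returns it to stunned.
; While ragdolled, Tick moves the actor to the spine and scales joint motor springs with hip speed.
; StopRagdoll realigns the capsule to hips and head and saves a pose snapshot for animation.
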(event `self.ReceiveBeginPlay`)

(event `self.ReceiveTick`
  (params (DeltaSeconds :type "Float (single-precision)"))
  (if (`self.GetIsRagdoll`)
    (`self.UpdateRagdoll`)))

(event `self.ReceiveActorBeginOverlap`
  (params (OtherActor :type "Actor Object Reference")))

(event `self.ReceiveAnyDamage`
  (params (Damage :type "Float (single-precision)") (DamageType :type "DamageType Object Reference") (InstigatedBy :type "Controller Object Reference") (DamageCauser :type "Actor Object Reference"))
  (bind _corpsetags (`self.CorpseTags`))
  (if (not (`BlueprintGameplayTagLibrary.HasTag` (`self.CorpseTags`) (struct :`TagName` "State.Corpse.Dragged")))
    (`BlueprintGameplayTagLibrary.RemoveGameplayTag` _corpsetags (struct :`TagName` "State.Corpse.GettingOut"))
    (`BlueprintGameplayTagLibrary.RemoveGameplayTag` _corpsetags (struct :`TagName` "State.Corpse.Waking"))
    (`BlueprintGameplayTagLibrary.RemoveGameplayTag` _corpsetags (struct :`TagName` "State.Corpse.Recovery"))
    (`BlueprintGameplayTagLibrary.AddGameplayTag` (`self.CorpseTags`) (struct :`TagName` "State.Corpse.Stunned"))))

(event `StartBeingDragged`
  (bind _corpsetags (`self.CorpseTags`))
  (`BlueprintGameplayTagLibrary.RemoveGameplayTag` _corpsetags (struct :`TagName` "State.Corpse.Stunned"))
  (`BlueprintGameplayTagLibrary.AddGameplayTag` _corpsetags (struct :`TagName` "State.Corpse.Dragged")))

(event `StopBeingDragged`
  (bind _corpsetags (`self.CorpseTags`))
  (`BlueprintGameplayTagLibrary.RemoveGameplayTag` _corpsetags (struct :`TagName` "State.Corpse.Dragged"))
  (`BlueprintGameplayTagLibrary.AddGameplayTag` _corpsetags (struct :`TagName` "State.Corpse.Stunned"))
  (`KismetSystemLibrary.PrintString` (`BlueprintGameplayTagLibrary.GetDebugStringFromGameplayTagContainer` (`self.CorpseTags`))))

(fn `EndRagdoll`)

(fn `Get Ragdoll Info`
  (returns (isRagdoll :type Boolean) (RagdollVelocity :type "Vector Structure"))
  (return (`self.GetIsRagdoll`) (`self.GetRagdollVelocity`)))

(fn `GetIsRagdoll`
  (returns (IsRagDoll :type Boolean))
  (return (`SceneComponent.IsSimulatingPhysics` (`self.Mesh`) "Hips")))

(fn `GetRagdollVelocity`
  (returns (ReturnValue :type "Vector Structure"))
  (bind _returnvalue (`SkeletalMeshComponent.GetBoneLinearVelocity` (`self.Mesh`) "Hips"))
  (return _returnvalue))

(fn `StartRagdoll`
  (bind _mesh (`self.Mesh`))
  (`|ExecutionSequence`
    (:`then_0`
      (`MovementComponent.StopMovementImmediately` (`self.CharacterMovement`))
      (`PrimitiveComponent.SetCollisionEnabled` (`self.CapsuleComponent`) "NoCollision")
      (`CharacterMovementComponent.SetMovementMode` (`self.CharacterMovement`) "MOVE_None" 0)
      (`PrimitiveComponent.SetCollisionObjectType` _mesh "ECC_PhysicsBody")
      (`PrimitiveComponent.SetCollisionEnabled` _mesh "QueryAndPhysics")
      (`PrimitiveComponent.SetSimulatePhysics` (`self.Mesh`) true))
    (:`then_1`
      (`self.UpdateRagdoll`))))

(fn `StopRagdoll`
  (bind _mesh (`self.Mesh`))
  (bind _capsulecomponent (`self.CapsuleComponent`))
  (bind _mesh_2 (`self.Mesh`))
  (bind (_returnvalue_x _returnvalue_y _returnvalue_z) (`KismetMathLibrary.BreakVector` (`SceneComponent.GetSocketLocation` (`self.Mesh`) "Hips")))
  (`SceneComponent.K2_SetWorldLocationAndRotation` _capsulecomponent (`KismetMathLibrary.MakeVector` _returnvalue_x _returnvalue_y (+ _returnvalue_z (`CapsuleComponent.CapsuleHalfHeight` _capsulecomponent))) (`KismetMathLibrary.MakeRotator` 0.0 0.0 (.yaw (`KismetMathLibrary.FindLookAtRotation` (`SceneComponent.GetSocketLocation` _mesh_2 "Hips") (`SceneComponent.GetSocketLocation` _mesh_2 "Head")))) false false)
  (`SceneComponent.K2_AttachToComponent` (`self.Mesh`) (`self.CapsuleComponent`) "None" "SnapToTarget" "SnapToTarget" "KeepRelative" true)
  (`AnimInstance.SavePoseSnapshot` (`SkeletalMeshComponent.GetAnimInstance` _mesh) "SavedRagdollPose")
  (`SceneComponent.K2_SetRelativeLocationAndRotation` _mesh (0.0 0.0 -90.0) (struct :`Yaw` -90.0) true true)
  (`PrimitiveComponent.SetSimulatePhysics` (`self.Mesh`) false)
  (`PrimitiveComponent.SetCollisionEnabled` (`self.CapsuleComponent`) "QueryAndPhysics")
  (`CharacterMovementComponent.SetMovementMode` (`self.CharacterMovement`) "MOVE_Falling" 0))

(fn `UpdateRagdoll`
  (`self.K2_SetActorLocationAndRotation` (+ (.location (`SceneComponent.GetSocketTransform` (`self.Mesh`) "Spine" "RTS_World")) (0.0 0.0 90.0)))
  (`SkeletalMeshComponent.SetAllMotorsAngularDriveParams` (`self.Mesh`) (`KismetMathLibrary.MapRangeClamped` (`KismetMathLibrary.VSize` (`self.GetRagdollVelocity`)) 0.0 500.0 500.0 5000.0) 0.0 0.0 false))

(fn `UserConstructionScript`)