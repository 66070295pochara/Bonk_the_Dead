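; BP_Spawner is a grave actor that removes its own corpses when they are brought back to it.
; On Box overlap it checks a BP_Corpse's gameplay tags for the Dragged or Stunned state, then destroys the corpse if its HomeGrave is this actor.
; Despite the name, no spawning logic lives in this graph, and its debug prints are disconnected.
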(event `self.ReceiveBeginPlay`)

(event `self.ReceiveActorBeginOverlap`
  (params (OtherActor :type "Actor Object Reference")))

(event `self.Box.OnComponentBeginOverlap`
  (params (OverlappedComponent :type "PrimitiveComponent Object Reference") (OtherActor :type "Actor Object Reference") (OtherComp :type "PrimitiveComponent Object Reference") (OtherBodyIndex :type Integer) (bFromSweep :type Boolean) (SweepResult :type "HitResult Structure (by ref)"))
  (bind _asbp_corpse (cast `/Game/Blueprint/BP_Corpse` OtherActor))
  (bind _corpsetags (`/Game/Blueprint/BP_Corpse.CorpseTags` _asbp_corpse))
  (if (or (`BlueprintGameplayTagLibrary.HasTag` _corpsetags (struct :`TagName` "State.Corpse.Dragged")) (`BlueprintGameplayTagLibrary.HasTag` _corpsetags (struct :`TagName` "State.Corpse.Stunned")))
    (if (== (`/Game/Blueprint/BP_Corpse.HomeGrave` _asbp_corpse) self)
      (`self.K2_DestroyActor` _asbp_corpse))))

(fn `UserConstructionScript`)