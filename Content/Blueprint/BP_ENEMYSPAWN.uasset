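; BP_ENEMYSPAWN is an enemy spawner actor that creates BP_Corpse actors at its own location and takes them back in when they return.
; A looping timer started on BeginPlay spawns a corpse every few seconds.
; When a corpse leaves its overlap area, a short delay sets its Canreturn flag.
; A flagged corpse that overlaps the spawner again is destroyed after a brief delay.
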(event `self.ReceiveBeginPlay`
  (`KismetSystemLibrary.K2_SetTimerDelegate` (delegate `spawn enemy`) 5.0 true))

(event `spawn enemy`
  (`|SpawnActorFromClass` "/Game/Blueprint/BP_Corpse.BP_Corpse_C" (`self.GetTransform`) "Undefined" "MultiplyWithRoot" null null))

(event `self.ReceiveActorEndOverlap`
  (params (OtherActor :type "Actor Object Reference"))
  (bind _asbp_corpse (cast `/Game/Blueprint/BP_Corpse` OtherActor))
  (`KismetSystemLibrary.Delay` 2.0)
  (set `/Game/Blueprint/BP_Corpse.canreturn` true _asbp_corpse))

(event `self.ReceiveActorBeginOverlap`
  (params (OtherActor :type "Actor Object Reference"))
  (bind _asbp_corpse (cast `/Game/Blueprint/BP_Corpse` OtherActor))
  (if (`/Game/Blueprint/BP_Corpse.canreturn` _asbp_corpse)
    (`KismetSystemLibrary.Delay` 1.0)
    (`self.K2_DestroyActor` _asbp_corpse)))

(fn `UserConstructionScript`)