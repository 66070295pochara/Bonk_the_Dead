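; BP_ShovelGameMode is the game mode that runs a three-night progression and decides win or loss.
; StartNight sets a timer whose length depends on the current night, and OnNightEnd advances the night, restarting the timer or printing a win after night three.
; EscapeCount increments the escape tally in BP_ShovelGameState and prints game over once the maximum is reached.
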(event `self.ReceiveBeginPlay`
  (`self.StartNight`))

(event `EscapeCount`
  (bind _asbp_shovel_game_state (cast `/Game/Core/BP_ShovelGameState` (`GameplayStatics.GetGameState`)))
  (set `/Game/Core/BP_ShovelGameState.Escaped` (+ (`/Game/Core/BP_ShovelGameState.Escaped` _asbp_shovel_game_state) 1) _asbp_shovel_game_state)
  (if (>= (`/Game/Core/BP_ShovelGameState.Escaped` _asbp_shovel_game_state) (`/Game/Core/BP_ShovelGameState.MaxEscaped` _asbp_shovel_game_state))
    (`KismetSystemLibrary.PrintString` "Game Over")))

(event `StartNight`
  (bind _asbp_shovel_game_state (cast `/Game/Core/BP_ShovelGameState` (`GameplayStatics.GetGameState`)))
  (bind _currentnight (`/Game/Core/BP_ShovelGameState.CurrentNight` _asbp_shovel_game_state))
  (switch `int` _currentnight
    (:`1`
      _)
    (:`2`
      _)
    (:`3`
      _))
  (bind _returnvalue (`KismetSystemLibrary.K2_SetTimerDelegate` (delegate `OnNightEnd`) (select `int` _currentnight :`0` 0.0 :`1` 5.0 :`2` 5.0 :`3` 10.0 :!type "Float (single-precision)")))
  (set `self.GameTime` _returnvalue))

(event `OnNightEnd`
  (bind _asbp_shovel_game_state (cast `/Game/Core/BP_ShovelGameState` (`GameplayStatics.GetGameState`)))
  (bind _currentnight (`/Game/Core/BP_ShovelGameState.CurrentNight` _asbp_shovel_game_state))
  (set `/Game/Core/BP_ShovelGameState.CurrentNight` (+ _currentnight 1) _asbp_shovel_game_state)
  (if (> _currentnight 3)
    (`KismetSystemLibrary.PrintString` "Win")
    (else
      (`self.StartNight`))))

(fn `UserConstructionScript`)