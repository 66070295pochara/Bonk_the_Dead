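; BP_Enemy is an enemy character, apparently a zombie, that reacts to damage and dies when its health runs out.
; AnyDamage subtracts from Health and sets IsDead when it reaches zero or below.
; A surviving hit plays a hit montage and launches the enemy away from the damage causer, overriding its velocity.
; A lethal hit passes a DoOnce to play the death montage once and stop movement immediately.
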(event `self.ReceiveAnyDamage`
  (params (Damage :type "Float (single-precision)") (DamageType :type "DamageType Object Reference") (InstigatedBy :type "Controller Object Reference") (DamageCauser :type "Actor Object Reference"))
  (set `self.Health` (- (`self.Health`) Damage))
  (set `self.isDead` (<= (`self.Health`) 0.0))
  (if (`self.isDead`)
    (`/Engine/EditorBlueprintResources/StandardMacros.DoOnce` false
      (:`Completed`
        (`|PlayMontage` (`self.Mesh`) "/Game/shovel/animation/AM_DEAD.AM_DEAD"
          (:`then`
            (`MovementComponent.StopMovementImmediately` (`self.CharacterMovement`))))))
    (else
      (`|PlayMontage` (`self.Mesh`) "/Game/shovel/animation/AM_ZOMBIE_HIT.AM_ZOMBIE_HIT"
        (:`then`
          (`self.LaunchCharacter` (* (`KismetMathLibrary.Normal` (- (`self.K2_GetActorLocation`) (`self.K2_GetActorLocation` DamageCauser)) 1.0) 2000.0) true true))))))

(fn `UserConstructionScript`)