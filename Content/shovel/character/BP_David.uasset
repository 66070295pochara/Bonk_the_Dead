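; First-person player character David, who fights with a shovel, drags physics bodies such as corpses with a spell and shoots tagged targets.
; BeginPlay attaches the shovel and adds HUD widgets; a hidden-head body and shadow-casting mesh play montages in parallel.
; A three-step montage combo uses notifies to trigger sphere-trace damage and open chaining.
; The spell hides the weapon, line-traces, then holds bodies camera-relative through a PhysicsHandle update loop.
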(event `spell`
  (bind _camera (`self.Camera`))
  (bind _returnvalue (`SceneComponent.K2_GetComponentLocation` _camera))
  (`|PlayMontage` (`self.Mesh`) "/Game/shovel/animation/AM_switchtohand.AM_switchtohand"
    (:`then`
      (`|PlayMontage` (`self.ShadowMesh`) "/Game/shovel/animation/AM_switchtohand.AM_switchtohand"
        (:`then`
          (`self.SetActorHiddenInGame` (`self.currentweapon`) true)
          (`self.SetActorEnableCollision` (`self.currentweapon`) false)
          (bind (_outhit _returnvalue_2) (`KismetSystemLibrary.LineTraceSingleForObjects` :`Start` _returnvalue :`End` (+ _returnvalue (* (`SceneComponent.GetForwardVector` _camera) 500.0)) :`ObjectTypes` (`|MakeArray` "ObjectTypeQuery4" :!type "EObjectTypeQuery Enum") :`DrawDebugType` "ForDuration"))
          (if _returnvalue_2
            (bind (_bblockinghit _binitialoverlap _time _distance _location _impactpoint _normal _impactnormal _physmat _hitactor _hitcomponent _hitbonename) (`GameplayStatics.BreakHitResult` _outhit))
            (bind _output_get (set `self.Drag_target_loc` _impactpoint))
            (bind _output_get_2 (set `self.drag_target` _hitcomponent))
            (`PhysicsHandleComponent.GrabComponentAtLocation` (`self.PhysicsHandle`) _output_get_2 _hitbonename _output_get)
            ; Start Dragged State
            (bind _asbp_corpse (cast `/Game/Blueprint/BP_Corpse` _hitactor))
            (`/Game/Blueprint/BP_Corpse.StartBeingDragged` _asbp_corpse)
            (`|PlayMontage` (`self.Mesh`) "/Game/shovel/animation/AM_SPELL.AM_SPELL"
              (:`then`
                (`|PlayMontage` (`self.ShadowMesh`) "/Game/shovel/animation/AM_SPELL.AM_SPELL"
                  (:`then`
                    (set `self.Drag_target_loc` (`KismetMathLibrary.InverseTransformLocation` (`SceneComponent.K2_GetComponentToWorld` (`self.Camera`)) (`self.Drag_target_loc`)))
                    (set `self.grabing` true)
                    (`self.update_drag_log`)))))
            (else
              (set `self.grabing` true)
              (`|PlayMontage` (`self.Mesh`) "/Game/shovel/animation/AM_SPELL.AM_SPELL"
                (:`then`
                  (`|PlayMontage` (`self.ShadowMesh`) "/Game/shovel/animation/AM_SPELL.AM_SPELL"))))))))))

(event `self.ReceiveTick`
  (params (DeltaSeconds :type "Float (single-precision)"))
  (`KismetSystemLibrary.PrintString` (`KismetStringLibrary.Conv_BoolToString` (`self.isattack`))))

(event `self.ReceiveBeginPlay`
  (bind _asplayer_controller (cast `PlayerController` (`GameplayStatics.GetPlayerController` 0)))
  (message `EnhancedInputSubsystemInterface.AddMappingContext` (pcsubsystem `EnhancedInputLocalPlayerSubsystem` _asplayer_controller) "/Game/shovel/input/IMC_DAVID.IMC_DAVID" 0 (struct))
  (bind _returnvalue (`|SpawnActorFromClass` "/Game/shovel/shovel0/BP_SHOVEL.BP_SHOVEL_C" (`SceneComponent.GetSocketTransform` (`self.Mesh`) "RH_weapon" "RTS_World") "Undefined" "MultiplyWithRoot" null null))
  (set `self.shovel_weapon` _returnvalue)
  (set `self.currentweapon` _returnvalue)
  (set `self.enum_weapon` "NewEnumerator1")
  (`self.K2_AttachToComponent` _returnvalue (`self.Mesh`) "RH_weapon" "SnapToTarget" "SnapToTarget" "SnapToTarget" true)
  (`PrimitiveComponent.SetCastHiddenShadow` (`self.ShadowMesh`) true)
  (`SkinnedMeshComponent.HideBoneByName` (`self.Mesh`) "Head" "PBO_None")
  (set `self.animation_instance` (`SkeletalMeshComponent.GetAnimInstance` (`self.Mesh`)))
  (bind _returnvalue_2 (`|CreateWidget` "/Game/Guns/Crosshair.Crosshair_C"))
  (`UserWidget.AddToViewport` _returnvalue_2 0)
  (bind _returnvalue_3 (`|CreateWidget` "/Game/grave/WB_Score.WB_Score_C"))
  (`UserWidget.AddToViewport` _returnvalue_3 0))

(event `CallAttackTrace`
  (bind _returnvalue (`SceneComponent.K2_GetComponentLocation` (`/Game/shovel/shovel0/BP_SHOVEL.StaticMesh` (`self.shovel_weapon`))))
  ; Apply damage
  (bind (_outhits _returnvalue_2) (`KismetSystemLibrary.SphereTraceMultiForObjects` :`Start` _returnvalue :`End` _returnvalue :`Radius` 50.0 :`ObjectTypes` (`|MakeArray` "ObjectTypeQuery3" :!type "EObjectTypeQuery Enum") :`DrawDebugType` "ForDuration"))
  (if _returnvalue_2
    (for _array_element _outhits
      (`GameplayStatics.ApplyDamage` (`.HitActor` (`GameplayStatics.BreakHitResult` _array_element)) 100.0 null self))))

(event `EnhancedInput|/Game/shovel/input/IA_DRAG`
  (params (ActionValue :type Boolean) (ElapsedSeconds :type "Float (double-precision)") (TriggeredSeconds :type "Float (double-precision)") (InputAction :type "InputAction Object Reference" :default "/Game/shovel/input/IA_DRAG.IA_DRAG"))
  (:`Started`
    (`self.spell`))
  (:`Canceled`
    (set `self.grabing` false :!label _label)
    (if (== (`self.currentweapon`) null)
      (`PhysicsHandleComponent.ReleaseComponent` (`self.PhysicsHandle`))
      ; Stop Dragged State
      (bind _output_get (set `self.drag_target` null))
      (bind _asbp_corpse (cast `/Game/Blueprint/BP_Corpse` (`ActorComponent.GetOwner` _output_get)))
      (`/Game/Blueprint/BP_Corpse.StopBeingDragged` _asbp_corpse)
      (`self.StopAnimMontage` "/Game/shovel/animation/AM_SPELL.AM_SPELL")
      (`AnimInstance.Montage_Stop` (`SkeletalMeshComponent.GetAnimInstance` (`self.ShadowMesh`)) 0.0 "/Game/shovel/animation/AM_SPELL.AM_SPELL")
      (else
        (`PhysicsHandleComponent.ReleaseComponent` (`self.PhysicsHandle`))
        (set `self.drag_target` null)
        (`self.StopAnimMontage` "/Game/shovel/animation/AM_SPELL.AM_SPELL")
        (`AnimInstance.Montage_Stop` (`SkeletalMeshComponent.GetAnimInstance` (`self.ShadowMesh`)) 0.0 "/Game/shovel/animation/AM_SPELL.AM_SPELL")
        (`self.SetActorHiddenInGame` (`self.currentweapon`) false)
        (`self.SetActorEnableCollision` (`self.currentweapon`) true))))
  (:`Completed`
    (goto _label)))

(event `EnhancedInput|/Game/shovel/input/IA_LOOK1`
  (params (ActionValue :type "Vector2D Structure") (ElapsedSeconds :type "Float (double-precision)") (TriggeredSeconds :type "Float (double-precision)") (InputAction :type "InputAction Object Reference" :default "/Game/shovel/input/IA_LOOK1.IA_LOOK1"))
  ; Comment
  (:`Triggered`
    (`self.AddControllerYawInput` ActionValue_X)
    (`self.AddControllerPitchInput` ActionValue_Y)))

(event `EnhancedInput|/Game/shovel/input/IA_MOVE1`
  (params (ActionValue :type "Vector2D Structure") (ElapsedSeconds :type "Float (double-precision)") (TriggeredSeconds :type "Float (double-precision)") (InputAction :type "InputAction Object Reference" :default "/Game/shovel/input/IA_MOVE1.IA_MOVE1"))
  ; Comment
  (:`Triggered`
    (`self.AddMovementInput` (`self.GetActorRightVector`) ActionValue_X)
    (`self.AddMovementInput` (`self.GetActorForwardVector`) ActionValue_Y)))

(event `EnhancedInput|/Game/shovel/input/IA_SHOVEL_ATTACK`
  (params (ActionValue :type Boolean) (ElapsedSeconds :type "Float (double-precision)") (TriggeredSeconds :type "Float (double-precision)") (InputAction :type "InputAction Object Reference" :default "/Game/shovel/input/IA_SHOVEL_ATTACK.IA_SHOVEL_ATTACK"))
  ; Combo Attack
  (:`Started`
    (if (`self.grabing`)
      _
      (elif (not (`self.isattack`))
        (switch `int` (`self.ComboIndex`)
          (:`0`
            (`|PlayMontage` (`self.Mesh`) "/Game/shovel/animation/AM_SHOVEL_ATTACK.AM_SHOVEL_ATTACK"
              (:`then`
                (bind _notifyname (`|PlayMontage` (`self.ShadowMesh`) "/Game/shovel/animation/AM_SHOVEL_ATTACK.AM_SHOVEL_ATTACK")
                  (:`then`
                    (set `self.isattack` true)
                    (set `self.ComboIndex` 1)
                    (`KismetSystemLibrary.PrintString` "Atack"))
                  (:`OnBlendOut`
                    (set `self.isattack` false :!label _label_2)
                    (`KismetSystemLibrary.RetriggerableDelay` 1.0)
                    (set `self.ComboIndex` 0))
                  (:`OnInterrupted`
                    (goto _label_2))
                  (:`OnNotifyBegin`
                    (switch `name` _notifyname
                      (:`AttackHit`
                        (`self.CallAttackTrace`))
                      (:`SaveAttack`
                        (set `self.isattack` false))))))))
          (:`1`
            (`|PlayMontage` (`self.Mesh`) "/Game/shovel/animation/AM_SHOVEL_SLAB.AM_SHOVEL_SLAB"
              (:`then`
                (bind _notifyname_2 (`|PlayMontage` (`self.ShadowMesh`) "/Game/shovel/animation/AM_SHOVEL_SLAB.AM_SHOVEL_SLAB")
                  (:`then`
                    (set `self.isattack` true)
                    (set `self.ComboIndex` 2)
                    (`KismetSystemLibrary.PrintString` "Slap"))
                  (:`OnBlendOut`
                    (set `self.isattack` false :!label _label_3)
                    (`KismetSystemLibrary.RetriggerableDelay` 1.0)
                    (set `self.ComboIndex` 0))
                  (:`OnInterrupted`
                    (goto _label_3))
                  (:`OnNotifyBegin`
                    (switch `name` _notifyname_2
                      (:`AttackHit`
                        (`self.CallAttackTrace`))
                      (:`SaveAttack`
                        (set `self.isattack` false))))))))
          (:`2`
            (`|PlayMontage` (`self.Mesh`) "/Game/shovel/animation/AM_AXE.AM_AXE"
              (:`then`
                (bind _notifyname_3 (`|PlayMontage` (`self.ShadowMesh`) "/Game/shovel/animation/AM_AXE.AM_AXE")
                  (:`then`
                    (set `self.isattack` true)
                    (set `self.ComboIndex` 0)
                    (`KismetSystemLibrary.PrintString` "heavy"))
                  (:`OnBlendOut`
                    (set `self.isattack` false :!label _label_4)
                    (`KismetSystemLibrary.RetriggerableDelay` 1.0)
                    (set `self.ComboIndex` 0))
                  (:`OnInterrupted`
                    (goto _label_4))
                  (:`OnNotifyBegin`
                    (switch `name` _notifyname_3
                      (:`AttackHit`
                        (`self.CallAttackTrace`))
                      (:`SaveAttack`
                        (set `self.isattack` false)))))))))))))

(event `Key|LeftShift`
  (params (Key :type "Key Structure"))
  (bind _charactermovement (`self.CharacterMovement`))
  ; run
  (:`Pressed`
    (if (not (`self.grabing`))
      (set `CharacterMovementComponent.MaxWalkSpeed` 600.0 _charactermovement)))
  (:`Released`
    (set `CharacterMovementComponent.MaxWalkSpeed` 300.0 _charactermovement)))

(event `EnhancedInput|/Game/shovel/input/IA_JUMP0`
  (params (ActionValue :type Boolean) (ElapsedSeconds :type "Float (double-precision)") (TriggeredSeconds :type "Float (double-precision)") (InputAction :type "InputAction Object Reference" :default "/Game/shovel/input/IA_JUMP0.IA_JUMP0"))
  ; Comment
  (:`Triggered`
    (`self.Jump`))
  (:`Completed`
    (`self.StopJumping`)))

(event `update_drag_log`
  (`/Engine/EditorBlueprintResources/StandardMacros.IsValid` (`self.drag_target`)
    (:`Is Valid`
      (`PhysicsHandleComponent.SetTargetLocation` (`self.PhysicsHandle`) (`KismetMathLibrary.TransformLocation` (`SceneComponent.K2_GetComponentToWorld` (`self.Camera`)) (`self.Drag_target_loc`)))
      (`KismetSystemLibrary.Delay` 0.01)
      (`self.update_drag_log`))))

(event `Key|One`
  (params (Key :type "Key Structure"))
  (:`Pressed`
    (if (not (`|EnumEquality` (`self.enum_weapon`) "NewEnumerator1"))
      (set `self.enum_weapon` "NewEnumerator1")
      (set `self.currentweapon` (`self.shovel_weapon`))
      (`|PlayMontage` (`self.Mesh`) "/Game/shovel/animation/AM_Switch.AM_Switch"
        (:`then`
          (`|PlayMontage` (`self.ShadowMesh`) "/Game/shovel/animation/AM_Switch.AM_Switch"
            (:`then`
              (`KismetSystemLibrary.Delay` 1.0)
              (`self.SetActorHiddenInGame` (`self.shovel_weapon`) false)
              (`self.SetActorEnableCollision` (`self.shovel_weapon`) true))))))))

(event `Key|NumPadTwo`
  (params (Key :type "Key Structure"))
  (:`Pressed`
    (set `self.enum_weapon` "NewEnumerator2")))

(event `EnhancedInput|/Game/Guns/IA_Shoot`
  (params (ActionValue :type Boolean) (ElapsedSeconds :type "Float (double-precision)") (TriggeredSeconds :type "Float (double-precision)") (InputAction :type "InputAction Object Reference" :default "/Game/Guns/IA_Shoot.IA_Shoot"))
  (bind _camera (`self.Camera`))
  (bind _returnvalue (+ (`SceneComponent.K2_GetComponentLocation` _camera) (0.0 0.0 -5.0)))
  (:`Triggered`
    (bind _outhit (`KismetSystemLibrary.LineTraceSingle` :`Start` _returnvalue :`End` (+ _returnvalue (* (`KismetMathLibrary.GetForwardVector` (`SceneComponent.K2_GetComponentRotation` _camera)) (3000.0 3000.0 3000.0))) :`TraceChannel` "TraceTypeQuery1" :`DrawDebugType` "ForDuration"))
    (bind (_bblockinghit _binitialoverlap _time _distance _location _impactpoint _normal _impactnormal _physmat _hitactor) (`GameplayStatics.BreakHitResult` _outhit))
    (if _bblockinghit
      (if (`self.ActorHasTag` _hitactor "CanShoot")
        (`self.K2_DestroyActor` _hitactor)
        (`KismetSystemLibrary.PrintString` "hit")
        (else
          (`KismetSystemLibrary.PrintString` "miss" :!label _label_5)))
      (else
        (goto _label_5)))))

(fn `check weapon`
  (if true
    _))

(fn `UserConstructionScript`
  (`SceneComponent.K2_AttachToComponent` (`self.Camera`) (`self.Mesh`) "neck_02" "KeepRelative" "KeepRelative" "KeepRelative" true))