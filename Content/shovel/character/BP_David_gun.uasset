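; First-person player character with a shovel and a gun, using Enhanced Input for movement and combat.
; Starts with the shovel; keys 1 and 2 spawn socket-attached weapons without removing previous ones.
; A three-step montage combo plays on body and shadow meshes, with notifies triggering sphere-trace damage and chaining.
; Shooting line-traces from the neck-attached camera independently of weapon mode, with delayed reloads from reserve ammo updating the HUD.
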(event `Key|One`
  (params (Key :type "Key Structure"))
  (:`Pressed`
    (set `self.WeaponMode` "NewEnumerator0" :!label _label)
    (bind _returnvalue (`|SpawnActorFromClass` "/Game/shovel/shovel0/BP_SHOVEL.BP_SHOVEL_C" (`SceneComponent.GetSocketTransform` (`self.Mesh`) "RH_weapon" "RTS_World") "Undefined" "MultiplyWithRoot" null null))
    (set `self.shovel_weapon` _returnvalue)
    (`self.K2_AttachToComponent` _returnvalue (`self.Mesh`) "RH_weapon" "SnapToTarget" "SnapToTarget" "SnapToTarget" true)
    (`PrimitiveComponent.SetCastHiddenShadow` (`self.ShadowMesh`) true)
    (`SkinnedMeshComponent.HideBoneByName` (`self.Mesh`) "Head" "PBO_None")
    (set `self.animation_instance` (`SkeletalMeshComponent.GetAnimInstance` (`self.Mesh`)))
    (bind _returnvalue_2 (`|CreateWidget` "/Game/Guns/Crosshair.Crosshair_C"))
    (`UserWidget.AddToViewport` _returnvalue_2 0)))

(event `EnhancedInput|/Game/Guns/IA_Reload`
  (params (ActionValue :type Boolean) (ElapsedSeconds :type "Float (double-precision)") (TriggeredSeconds :type "Float (double-precision)") (InputAction :type "InputAction Object Reference" :default "/Game/Guns/IA_Reload.IA_Reload"))
  ; Reload
  (:`Triggered`
    (set `self.isreloading` true)
    (`KismetSystemLibrary.PrintString` "Reloading")
    (`KismetSystemLibrary.Delay` 1.5)
    (bind _output_get (set `self.needAmmo` (- (`self.maxAmmo`) (`self.currentAmmo`))))
    (if (>= (`self.reserveAmmo`) _output_get)
      (set `self.currentAmmo` (`self.maxAmmo`))
      (set `self.reserveAmmo` (- (`self.reserveAmmo`) (`self.needAmmo`)))
      (else
        (set `self.currentAmmo` (+ (`self.currentAmmo`) (`self.reserveAmmo`)))
        (set `self.reserveAmmo` 0)))
    (`/Game/Guns/Ammo.UpdateAmmo` (`self.AmmoWidget`) (`self.currentAmmo`) (`self.reserveAmmo`))
    (set `self.isreloading` false)))

(event `self.ReceiveBeginPlay`
  (bind _asplayer_controller (cast `PlayerController` (`GameplayStatics.GetPlayerController` 0)))
  (message `EnhancedInputSubsystemInterface.AddMappingContext` (pcsubsystem `EnhancedInputLocalPlayerSubsystem` _asplayer_controller) "/Game/shovel/input/IMC_DAVID.IMC_DAVID" 0 (struct))
  (goto _label))

(event `CallAttackTrace`
  (bind _returnvalue (`SceneComponent.K2_GetComponentLocation` (`/Game/shovel/shovel0/BP_SHOVEL.StaticMesh` (`self.shovel_weapon`))))
  ; Apply damage
  (bind (_outhits _returnvalue_2) (`KismetSystemLibrary.SphereTraceMultiForObjects` :`Start` _returnvalue :`End` _returnvalue :`Radius` 50.0 :`ObjectTypes` (`|MakeArray` "ObjectTypeQuery3" :!type "EObjectTypeQuery Enum") :`DrawDebugType` "ForDuration"))
  (if _returnvalue_2
    (for _array_element _outhits
      (`GameplayStatics.ApplyDamage` (`.HitActor` (`GameplayStatics.BreakHitResult` _array_element)) 25.0 null self))))

(event `EnhancedInput|/Game/shovel/input/IA_LOOK1`
  (params (ActionValue :type "Vector2D Structure") (ElapsedSeconds :type "Float (double-precision)") (TriggeredSeconds :type "Float (double-precision)") (InputAction :type "InputAction Object Reference" :default "/Game/shovel/input/IA_LOOK1.IA_LOOK1"))
  ; Comment
  (:`Triggered`
    (`self.AddControllerYawInput` ActionValue_X)
    (`self.AddControllerPitchInput` ActionValue_Y)))

(event `EnhancedInput|/Game/shovel/input/IA_MOVE1`
  (params (ActionValue :type "Vector2D Structure") (ElapsedSeconds :type "Float (double-precision)") (TriggeredSeconds :type "Float (double-precision)") (InputAction :type "InputAction Object Reference" :default "/Game/shovel/input/IA_MOVE1.IA_MOVE1"))
  ; Comment
  (:`Triggered`
    (`self.AddMovementInput` (`self.GetActorRightVector`) ActionValue_X)
    (`self.AddMovementInput` (`self.GetActorForwardVector`) ActionValue_Y)))

(event `EnhancedInput|/Game/Guns/IA_Shoot`
  (params (ActionValue :type Boolean) (ElapsedSeconds :type "Float (double-precision)") (TriggeredSeconds :type "Float (double-precision)") (InputAction :type "InputAction Object Reference" :default "/Game/Guns/IA_Shoot.IA_Shoot"))
  (bind _camera (`self.Camera`))
  (bind _returnvalue (+ (`SceneComponent.K2_GetComponentLocation` _camera) (0.0 0.0 -5.0)))
  ; Gun Logic
  (:`Triggered`
    (if (`self.isreloading`)
      _
      (elif (> (`self.currentAmmo`) 0)
        (bind _outhit (`KismetSystemLibrary.LineTraceSingleForObjects` :`Start` _returnvalue :`End` (+ _returnvalue (* (`KismetMathLibrary.GetForwardVector` (`SceneComponent.K2_GetComponentRotation` _camera)) (3000.0 3000.0 3000.0))) :`ObjectTypes` (`|MakeArray` "ObjectTypeQuery3" :!type "EObjectTypeQuery Enum") :`DrawDebugType` "ForDuration"))
        (bind _output_get (set `self.currentAmmo` (- (`self.currentAmmo`) 1)))
        (`/Game/Guns/Ammo.UpdateAmmo` (`self.AmmoWidget`) _output_get (`self.reserveAmmo`))
        (bind (_bblockinghit _binitialoverlap _time _distance _location _impactpoint _normal _impactnormal _physmat _hitactor) (`GameplayStatics.BreakHitResult` _outhit))
        (if _bblockinghit
          (`GameplayStatics.ApplyDamage` _hitactor 40.0 null self)
          (`KismetSystemLibrary.PrintString` "hit")
          (else
            (`KismetSystemLibrary.PrintString` "miss")))
        (else
          (`KismetSystemLibrary.PrintString` "No Ammo"))))))

(event `EnhancedInput|/Game/shovel/input/IA_JUMP0`
  (params (ActionValue :type Boolean) (ElapsedSeconds :type "Float (double-precision)") (TriggeredSeconds :type "Float (double-precision)") (InputAction :type "InputAction Object Reference" :default "/Game/shovel/input/IA_JUMP0.IA_JUMP0"))
  ; Comment
  (:`Triggered`
    (`self.Jump`))
  (:`Completed`
    (`self.StopJumping`)))

(event `Key|Two`
  (params (Key :type "Key Structure"))
  ; Equip gun
  (:`Pressed`
    (set `self.WeaponMode` "NewEnumerator1")
    (bind _returnvalue (`|SpawnActorFromClass` "/Game/Guns/BP_Gun.BP_Gun_C" (`SceneComponent.GetSocketTransform` (`self.Mesh`) "RH_gun" "RTS_World") "Undefined" "MultiplyWithRoot" null null))
    (set `self.gun_weapon` _returnvalue)
    (`self.K2_AttachToComponent` _returnvalue (`self.Mesh`) "RH_gun" "SnapToTarget" "SnapToTarget" "SnapToTarget" true)
    (`PrimitiveComponent.SetCastHiddenShadow` (`self.ShadowMesh`) true)
    (`SkinnedMeshComponent.HideBoneByName` (`self.Mesh`) "Head" "PBO_None")
    (set `self.animation_instance` (`SkeletalMeshComponent.GetAnimInstance` (`self.Mesh`)))
    (bind _returnvalue_2 (`|CreateWidget` "/Game/Guns/Crosshair.Crosshair_C"))
    (bind _returnvalue_3 (`|CreateWidget` "/Game/Guns/Ammo.Ammo_C"))
    (bind _output_get (set `self.AmmoWidget` _returnvalue_3))
    (`/Game/Guns/Ammo.UpdateAmmo` _output_get (`self.currentAmmo`) (`self.maxAmmo`))
    (`UserWidget.AddToViewport` _returnvalue_2 0)
    (`UserWidget.AddToViewport` _output_get 0)))

(event `EnhancedInput|/Game/shovel/input/IA_SHOVEL_ATTACK`
  (params (ActionValue :type Boolean) (ElapsedSeconds :type "Float (double-precision)") (TriggeredSeconds :type "Float (double-precision)") (InputAction :type "InputAction Object Reference" :default "/Game/shovel/input/IA_SHOVEL_ATTACK.IA_SHOVEL_ATTACK"))
  ; Combo Attack
  (:`Started`
    (if (not (`self.isattack`))
      (switch `int` (`self.ComboIndex`)
        (:`0`
          (`|PlayMontage` (`self.Mesh`) "/Game/shovel/animation/AM_SHOVEL_ATTACK.AM_SHOVEL_ATTACK"
            (:`then`
              (bind _notifyname (`|PlayMontage` (`self.ShadowMesh`) "/Game/shovel/animation/AM_SHOVEL_ATTACK.AM_SHOVEL_ATTACK")
                (:`then`
                  (set `self.isattack` true)
                  (set `self.ComboIndex` 1)
                  (`KismetSystemLibrary.PrintString` "Atack"))
                (:`OnBlendOut`
                  (set `self.isattack` false)
                  (`KismetSystemLibrary.RetriggerableDelay` 1.0)
                  (set `self.ComboIndex` 0))
                (:`OnNotifyBegin`
                  (switch `name` _notifyname
                    (:`AttackHit`
                      (`self.CallAttackTrace`))
                    (:`SaveAttack`
                      (set `self.isattack` false))))))))
        (:`1`
          (`|PlayMontage` (`self.Mesh`) "/Game/shovel/animation/AM_SHOVEL_SLAB.AM_SHOVEL_SLAB"
            (:`then`
              (bind _notifyname_2 (`|PlayMontage` (`self.ShadowMesh`) "/Game/shovel/animation/AM_SHOVEL_SLAB.AM_SHOVEL_SLAB")
                (:`then`
                  (set `self.isattack` true)
                  (set `self.ComboIndex` 2)
                  (`KismetSystemLibrary.PrintString` "Slap"))
                (:`OnBlendOut`
                  (set `self.isattack` false)
                  (`KismetSystemLibrary.RetriggerableDelay` 1.0)
                  (set `self.ComboIndex` 0))
                (:`OnNotifyBegin`
                  (switch `name` _notifyname_2
                    (:`AttackHit`
                      (`self.CallAttackTrace`))
                    (:`SaveAttack`
                      (set `self.isattack` false))))))))
        (:`2`
          (`|PlayMontage` (`self.Mesh`) "/Game/shovel/animation/AM_AXE.AM_AXE"
            (:`then`
              (bind _notifyname_3 (`|PlayMontage` (`self.ShadowMesh`) "/Game/shovel/animation/AM_AXE.AM_AXE")
                (:`then`
                  (set `self.isattack` true)
                  (set `self.ComboIndex` 0)
                  (`KismetSystemLibrary.PrintString` "heavy"))
                (:`OnBlendOut`
                  (set `self.isattack` false)
                  (`KismetSystemLibrary.RetriggerableDelay` 1.0)
                  (set `self.ComboIndex` 0))
                (:`OnNotifyBegin`
                  (switch `name` _notifyname_3
                    (:`AttackHit`
                      (`self.CallAttackTrace`))
                    (:`SaveAttack`
                      (set `self.isattack` false))))))))))))

(fn `UserConstructionScript`
  (`SceneComponent.K2_AttachToComponent` (`self.Camera`) (`self.Mesh`) "neck_02" "KeepRelative" "KeepRelative" "KeepRelative" true))